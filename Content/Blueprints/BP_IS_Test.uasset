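; Test Blueprint for streaming text-to-speech with the InoSherpa plugin and a Piper English voice.
; On BeginPlay it loads the model from hard-coded placeholder paths, prints the result and creates a streaming sound wave.
; Handlers append synthesized Int16 audio to the wave and play it once on its first populate event.
; The async synthesis call and populate binding are disconnected, so no speech plays.
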(event Custom|CustomEvent
  (params (Result :type Ino%20TTS%20Result%20Structure%20%28by%20ref%29))
  (bind (_bsuccess _errormessage _audiosamples _samplerate _numchannels) (Utilities|Struct|BreakInoTTSResult Result))
  (if _bsuccess
    (Class|StreamingSoundWave|AppendAudioDatafromRAW (Variables|Default|GetSoundWaveStream) _audiosamples "Int16" _samplerate _numchannels)
    (else
      (Development|PrintString _errormessage true true "(R=0.000000,G=0.660000,B=1.000000,A=1.000000)" 2e+01))))

(event Custom|OnPopulateAudioState_Event
  (Utilities|FlowControl|DoOnce false
    (:Completed
      (Audio|PlaySound2D (Variables|Default|GetSoundWaveStream) 1.0 1.0 0.0 0 0))))

(event EventBeginPlay
  (bind (_outerror _returnvalue) (Class|InoTTS|LoadModel (Subsystems|GetInoTTS) (Utilities|Struct|MakeInoTTSModelConfig "PiperVits" (Utilities|Struct|MakeInoTTSPiperConfig "D:\\ModelsRoot\\EDIT_THIS_PATH_IN_EDITOR\\Plugins\\InoSherpa\\SherpaOnnx\\models\\vits-piper-en_US-libritts_r-medium\\en_US-libritts_r-medium.onnx" "D:\\ModelsRoot\\EDIT_THIS_PATH_IN_EDITOR\\Plugins\\InoSherpa\\SherpaOnnx\\models\\vits-piper-en_US-libritts_r-medium\\tokens.txt" "D:\\ModelsRoot\\EDIT_THIS_PATH_IN_EDITOR\\Plugins\\InoSherpa\\SherpaOnnx\\models\\vits-piper-en_US-libritts_r-medium\\espeak-ng-data"))))
  (Development|PrintString (Utilities|String|Append (Utilities|String|ToString(Boolean) _returnvalue) " : " _outerror) true true "(R=0.000000,G=0.660000,B=1.000000,A=1.000000)" 2e+01)
  (bind _returnvalue_2 (Class|StreamingSoundWave|CreateStreamingSoundWave))
  (Variables|Default|SetSoundWaveStream _returnvalue_2))

(fn ConstructionScript)